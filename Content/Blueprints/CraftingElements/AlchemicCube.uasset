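; AlchemicCube is an alchemy crafting prop whose burners and candle the player lights with a tinder-box.
; Start checks the character's Trutnici array, then once calls svech, changes collision, plays a match sound and shows lights and particles.
; A timeline drives both light intensities.
; Without enough tinder-boxes it shows a hand-widget message and resets the DoOnce, while ITM reports SVECHA as true.
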(event EventStart
  (params (char :type Third%20Person%20Character%20Osnova%20Object%20Reference))
  (bind _rucawidget (Variables|/Game/Character_BP/AnimCharacter/HeroCharacters/ThirdPersonCharacterOsnova.ThirdPersonCharacterOsnova_C|GetRucaWidget char))
  (bind _pointlight (Variables|Default|GetPointLight))
  (bind _hand_wid (Variables|/Game/AICharacter_BP/AISystem/widhad.widhad_C|GetHand_wid _rucawidget))
  (if (> (Utilities|Array|LastIndex (Variables|/Game/Character_BP/AnimCharacter/HeroCharacters/ThirdPersonCharacterOsnova.ThirdPersonCharacterOsnova_C|GetTrutnici char)) 0)
    (Utilities|FlowControl|DoOnce false :!label _label
      (:Completed
        (Default|-svech char "NewEnumerator0")
        (Collision|SetCollisionObjectType (Variables|Default|GetSM_Burner-02) "ECC_WorldStatic")
        (Audio|PlaySoundatLocation "/Game/SFXInteraction/Wav/set_fire_to_a_match2.set_fire_to_a_match2" "0, 0, 0" "0, 0, 0" 1.0 1.0 0.0 0 0 0)
        (Rendering|SetVisibility _pointlight true false)
        (bind (_direction _light1 _light) (Timeline|Lighting Play)
          (:Update
            (Rendering|Components|Light|SetIntensity _pointlight _light1)
            (Rendering|Components|Light|SetIntensity (Variables|Default|GetPointLight1) _light)
            (Rendering|SetVisibility (Variables|Default|GetParticleSystem) true false)))))
    (else
      (Rendering|Components|TextRender|SetText (Variables|/Game/AICharacter_BP/AISystem/Hand_wid.Hand_wid_C|GetText _hand_wid) "No Tinder-boxes left")
      (Default|ActivateAnimation _hand_wid)
      (goto _label Reset))))

(fn ConstructionScript)

(fn ITM
  (return 0 true))