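; Smelting furnace actor that turns ore and a placed casting mold into a spawned Gear.
; Overlaps install the mold and, once the child FurnacePotTrigger reports coal (Ygol), consume ore up to a target count.
; Chained timelines with delays then animate pouring metal by scaling and moving meshes, with sounds and particles, before the Gear spawns.
; An outer overlap sphere shows missing-mold or no-fire warning widgets, destroying itself when both conditions are met.
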(event OnComponentBeginOverlap(Sphere1)
  (params (OverlappedComponent :type Primitive%20Component%20Object%20Reference) (OtherActor :type Actor%20Object%20Reference) (OtherComp :type Primitive%20Component%20Object%20Reference) (OtherBodyIndex :type Integer) (bFromSweep :type Boolean) (SweepResult :type Hit%20Result%20Structure%20%28by%20ref%29))
  (bind _pechwidget (Variables|Default|GetPechWidget))
  (bind _pechwidget1 (Variables|Default|GetPechWidget1))
  (Utilities|Casting|CastToOre OtherActor)
  (if (Variables|Default|GetForma)
    (if (Variables|Default|GetYgol)
      (Components|DestroyComponent (Variables|Default|GetSphere1))
      (else
        (UserInterface|Viewport|AddtoViewport _pechwidget1 0)
        (Utilities|FlowControl|Delay 1.5)
        (Widget|RemovefromParent _pechwidget1)))
    (else
      (UserInterface|Viewport|AddtoViewport _pechwidget 0)
      (Utilities|FlowControl|Delay 1.5)
      (Widget|RemovefromParent _pechwidget))))

(event OnComponentBeginOverlap(Box)
  (params (OverlappedComponent :type Primitive%20Component%20Object%20Reference) (OtherActor :type Actor%20Object%20Reference) (OtherComp :type Primitive%20Component%20Object%20Reference) (OtherBodyIndex :type Integer) (bFromSweep :type Boolean) (SweepResult :type Hit%20Result%20Structure%20%28by%20ref%29))
  ;[1 1 1] Форма
  (bind _asforma (Utilities|Casting|CastToforma OtherActor))
  (Rendering|SetVisibility (Variables|Default|GetCopperGearForm1) true false)
  (Audio|PlaySoundatLocation "/Game/Sounds/CustomPhysicsSounds/StoneForma/StoneFormaHit3.StoneFormaHit3" "0, 0, 0" "0, 0, 0" 1.0 1.0 0.0 0 0 0)
  (Variables|Default|SetForma true)
  (Actor|DestroyActor _asforma)
  (Variables|/Game/Blueprints/Resourses/FurnacePotTrigger.FurnacePotTrigger_C|SetForma (Variables|Default|GetAs%20Furnace%20Pot%20Trigger) true))

(event OnComponentBeginOverlap(Sphere)
  (params (OverlappedComponent :type Primitive%20Component%20Object%20Reference) (OtherActor :type Actor%20Object%20Reference) (OtherComp :type Primitive%20Component%20Object%20Reference) (OtherBodyIndex :type Integer) (bFromSweep :type Boolean) (SweepResult :type Hit%20Result%20Structure%20%28by%20ref%29))
  (bind _cylindermetal (Variables|Default|GetCylinderMetal))
  (bind _metaljidkiy (Variables|Default|GetMetalJidkiy))
  (bind _actor (Variables|Default|Getactor))
  (bind _spheremetaljidkiy (Variables|Default|GetSphereMetalJidkiy))
  (bind _cylindermetalreverse (Variables|Default|GetCylinderMetalReverse))
  (bind _returnvalue (Transformation|GetRelativeTransform _metaljidkiy))
  (bind _returnvalue_2 (Transformation|GetRelativeTransform _spheremetaljidkiy))
  ;[1 1 1] Подсчет Руды
  (bind _asore (Utilities|Casting|CastToOre OtherActor))
  (bind _drova_3 (Default|Ygol (Variables|Default|GetAs%20Furnace%20Pot%20Trigger)))
  (if _drova_3
    (Utilities|Array|Add _actor _asore)
    (Actor|DestroyActor _asore)
    (if (== (Utilities|Array|Length _actor) (Variables|Default|Getindxkod))
      (Utilities|Array|Clear _actor)
      (Variables|Default|SetMojnoPlavit true)
      (Utilities|FlowControl|Delay 2.0)
      (Components|Activation|Activate (Variables|Default|GetParticleSystem) true)
      (Rendering|SetVisibility _cylindermetal true false)
      (Audio|PlaySoundatLocation "/Game/Sounds/CustomSounds/Pech/LitieMetalla.LitieMetalla" "0, 0, 0" "0, 0, 0" 1.0 1.0 0.0 0 0 0)
      (Audio|PlaySoundatLocation "/Game/Sounds/CustomSounds/Pech/ZvukPara.ZvukPara" "0, 0, 0" "0, 0, 0" 1.0 1.0 0.0 0 0 0)
      (bind _metal (Timeline|CYLINDER Play)
        (:Update
          (Transformation|SetRelativeTransform _cylindermetal (Math|Transform|MakeTransform (.location (Transformation|GetRelativeTransform _cylindermetal)) "0, 0, 0" (Math|Vector|MakeVector 0.04 0.04 _metal)) false false)
          (Utilities|FlowControl|Sequence
            (:then_0
              (Utilities|FlowControl|Delay 1.75)
              (bind (_direction _metal_2 _z) (Timeline|MetalJidkiySphere Play)
                (:Update
                  (Rendering|SetVisibility _spheremetaljidkiy true false)
                  (Transformation|SetRelativeTransform _spheremetaljidkiy (Math|Transform|MakeTransform (Math|Vector|MakeVector (.x (.location _returnvalue_2)) (.y (.location _returnvalue_2)) _metal_2) (.rotation _returnvalue_2) (.scale _returnvalue_2)) false false)
                  (Rendering|SetVisibility _cylindermetalreverse true false)
                  (Utilities|FlowControl|Sequence
                    (:then_0
                      (Utilities|FlowControl|DoOnce false
                        (:Completed
                          (Audio|PlaySoundatLocation "/Game/Sounds/CustomSounds/Pech/MetalBrizg.MetalBrizg" "0, 0, 0" "0, 0, 0" 1.0 1.0 0.0 0 0 0))))
                    (:then_1
                      (Transformation|SetRelativeTransform _cylindermetalreverse (Math|Transform|MakeTransform (.location (Transformation|GetRelativeTransform _cylindermetalreverse)) "0, 0, 0" (Math|Vector|MakeVector 0.04 0.04 _z)) false false)
                      (Rendering|SetVisibility (Variables|Default|GetCylinderMetal) false false)
                      (Utilities|FlowControl|Delay 1.9)
                      (Rendering|SetVisibility _metaljidkiy true false)
                      (bind _z2 (Timeline|Jidkiy Play)
                        (:Update
                          (Transformation|SetRelativeTransform _metaljidkiy (Math|Transform|MakeTransform (Math|Vector|MakeVector (.x (.location _returnvalue)) (.y (.location _returnvalue)) _z2) "0, 0, 0" (.scale _returnvalue)) false false))
                        (:Finished
                          (Rendering|SetVisibility (Variables|Default|GetCylinderMetalReverse) false false)
                          (Components|Activation|Deactivate (Variables|Default|GetParticleSystem1))
                          (Utilities|FlowControl|DoOnce false
                            (:Completed
                              (Utilities|FlowControl|Delay 2.0)
                              (Rendering|SetVisibility (Variables|Default|GetSphereMetalJidkiy) false false)
                              (Rendering|SetVisibility (Variables|Default|GetMetalJidkiy) false false)
                              (Game|SpawnActorfromClass "/Game/Blueprints/Gear.Gear_C" (Math|Transform|MakeTransform (Transformation|GetWorldLocation (Variables|Default|GetScene)) "0, 0, 0" "1,1,1") "Undefined" 0 0))))))))))
            (:then_1
              (Utilities|FlowControl|Delay 1.35)
              (Utilities|FlowControl|DoOnce false
                (:Completed
                  (Audio|PlaySoundatLocation "/Game/Sounds/CustomSounds/Pech/MetalShipenie.MetalShipenie" "0, 0, 0" "0, 0, 0" 1.0 1.0 0.0 0 0 0)
                  (Components|Activation|Activate (Variables|Default|GetSmoke) false))))))))))

(event Custom|DeletePlane
  ;[1 1 1] Подсчет Руды
  (if (Variables|Default|GetForma)
    (Components|DestroyComponent (Variables|Default|GetPlane))))

(event EventBeginPlay
  ;[1 1 1] Печка
  (Utilities|FlowControl|Sequence
    (:then_0
      (bind _asfurnace_pot_trigger (Utilities|Casting|CastToFurnacePotTrigger (Variables|/Script/Engine.ChildActorComponent|GetChildActor (Variables|Default|GetFurnacePotTrigger))))
      (bind _output_get (Variables|Default|SetAs%20Furnace%20Pot%20Trigger _asfurnace_pot_trigger))
      (Variables|/Game/Blueprints/Resourses/FurnacePotTrigger.FurnacePotTrigger_C|SetPech _output_get self)
      (bind _asthird_person_character_osnova (Utilities|Casting|CastToThirdPersonCharacterOsnova (Game|GetPlayerCharacter 0)))
      (Variables|Default|SetAs%20Third%20Person%20Character%20Osnova _asthird_person_character_osnova)
      (bind _returnvalue (UserInterface|CreateWidget "/Game/Blueprints/Widgets/NoStoneCastWidget.NoStoneCastWidget_C"))
      (Variables|Default|SetPechWidget _returnvalue)
      (bind _returnvalue_2 (UserInterface|CreateWidget "/Game/Blueprints/Widgets/NoFireWidget.NoFireWidget_C"))
      (Variables|Default|SetPechWidget1 _returnvalue_2))
    (:then_1)))

(event EventTick
  (params (DeltaSeconds :type Float%20%28single-precision%29)))

(fn ConstructionScript)