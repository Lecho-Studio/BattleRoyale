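; Furnace firebox trigger that collects three wood logs and lets the player light them.
; Each overlapping log is replaced by a non-colliding copy snapped to one of three arrows, counted by a DoN.
; Start checks for logs, tinder-boxes and a stone cast, showing hand-widget messages if either of the latter is missing.
; Ignition runs once, spawning fire and coal, playing timeline-driven light and sound, and notifying the linked furnace (Pech).
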(event OnComponentBeginOverlap(Box)
  (params (OverlappedComponent :type Primitive%20Component%20Object%20Reference) (OtherActor :type Actor%20Object%20Reference) (OtherComp :type Primitive%20Component%20Object%20Reference) (OtherBodyIndex :type Integer) (bFromSweep :type Boolean) (SweepResult :type Hit%20Result%20Structure%20%28by%20ref%29))
  (bind _aswood_log (Utilities|Casting|CastToWoodLog OtherActor))
  (bind _counter (Utilities|FlowControl|DoN 3)
    (:Exit
      (if (== _counter 1)
        (Variables|Default|SetTarget (Variables|Default|GetArrow))
        (elif (== _counter 2)
          (Variables|Default|SetTarget (Variables|Default|GetArrow1))
          (elif (== _counter 3)
            (Variables|Default|SetTarget (Variables|Default|GetArrow2)))))
      (bind _returnvalue (Game|SpawnActorfromClass "/Game/Blueprints/Resourses/WoodLog.WoodLog_C" (Math|Transform|MakeTransform (.location (Transformation|GetWorldTransform (Variables|Default|GetTarget))) (Math|Rotator|MakeRotator (+ (.roll (.rotation (Transformation|GetWorldTransform (Variables|Default|GetTarget)))) 9e+01) (+ (.pitch (.rotation (Transformation|GetWorldTransform (Variables|Default|GetTarget)))) 9e+01) (+ (.yaw (.rotation (Transformation|GetWorldTransform (Variables|Default|GetTarget)))) 9e+01)) "1,1,1") "Undefined" 0 0))
      (Audio|PlaySoundatLocation "/Game/Sounds/CustomPhysicsSounds/WoodLog/Brewno_Cue.Brewno_Cue" "0, 0, 0" "0, 0, 0" 1.0 1.0 0.0 0 0 0)
      (bind _output_get (Variables|Default|SetDrova _returnvalue))
      (Utilities|Array|Add (Variables|Default|GetMassivDrov) _output_get)
      (Physics|SetSimulatePhysics (Variables|/Game/Blueprints/Resourses/WoodLog.WoodLog_C|GetStaticMesh _returnvalue) false)
      (Transformation|SetActorLocationAndRotation _returnvalue (.location (Transformation|GetWorldTransform (Variables|Default|GetTarget))) (Math|Rotator|MakeRotator (+ (.roll (.rotation (Transformation|GetWorldTransform (Variables|Default|GetTarget)))) 9e+01) (+ (.pitch (.rotation (Transformation|GetWorldTransform (Variables|Default|GetTarget)))) 9e+01) (+ (.yaw (.rotation (Transformation|GetWorldTransform (Variables|Default|GetTarget)))) 9e+01)))
      (Actor|DestroyActor _aswood_log)
      (Collision|SetCollisionEnabled (Variables|/Game/Blueprints/Resourses/WoodLog.WoodLog_C|GetStaticMesh _returnvalue) "NoCollision")
      (bind _output_get_2 (Variables|Default|SetDrovaNaMeste true))
      (Variables|Default|SetProverka%20Colichestva%20Drov (== _counter 3)))))

(event EventStart
  (params (char :type Third%20Person%20Character%20Osnova%20Object%20Reference))
  (bind _rucawidget (Variables|/Game/Character_BP/AnimCharacter/HeroCharacters/ThirdPersonCharacterOsnova.ThirdPersonCharacterOsnova_C|GetRucaWidget char))
  (bind _pech (Variables|Default|GetPech))
  (bind _arrowfirespawner (Variables|Default|GetArrowFireSpawner))
  (bind _pointlight1 (Variables|Default|GetPointLight1))
  (bind _returnvalue (Transformation|GetWorldLocation _arrowfirespawner))
  (bind _hand_wid (Variables|/Game/AICharacter_BP/AISystem/widhad.widhad_C|GetHand_wid _rucawidget))
  (bind _text (Variables|/Game/AICharacter_BP/AISystem/Hand_wid.Hand_wid_C|GetText _hand_wid))
  (if (== (stale OnComponentBeginOverlap(Box) _counter) 3)
    (if (stale OnComponentBeginOverlap(Box) _output_get_2)
      (if (> (Utilities|Array|LastIndex (Variables|/Game/Character_BP/AnimCharacter/HeroCharacters/ThirdPersonCharacterOsnova.ThirdPersonCharacterOsnova_C|GetTrutnici char)) 0)
        (if (Variables|Default|GetForma)
          (Utilities|FlowControl|DoOnce false :!label _label
            (:Completed
              (Default|-svech char "NewEnumerator0")
              (for _array_element (Variables|Default|GetMassivDrov)
                (Utilities|IsValid _array_element))
              (Variables|Default|SetDeactivate%20Widget true)
              (Effects|SpawnEmitteratLocation "/Game/Magic_Room/Particles/PS_Fire.PS_Fire" _returnvalue)
              (Utilities|FlowControl|Sequence
                (:then_0
                  (Utilities|FlowControl|DoOnce false
                    (:Completed
                      (Audio|PlaySoundatLocation "/Game/SFXInteraction/Wav/set_fire_to_a_match2.set_fire_to_a_match2" "0, 0, 0" "0, 0, 0" 1.0 1.0 0.0 0 0 0)
                      (Rendering|SetVisibility _pointlight1 true false)
                      (bind _lighting (Timeline|Timeline_0 Play)
                        (:Update
                          (Rendering|Components|Light|SetIntensity _pointlight1 _lighting)
                          (Utilities|FlowControl|Sequence
                            (:then_0
                              (Utilities|FlowControl|Delay 2.5)
                              (bind _newtrack_2 (Timeline|FireAnim Play)
                                (:Update
                                  (Rendering|Components|Light|SetIntensity (Variables|Default|GetPointLight1) _newtrack_2))))
                            (:then_1
                              (Utilities|FlowControl|DoOnce false
                                (:Completed
                                  (Components|Activation|Activate (Variables|Default|GetTorchLoop) false))))))))))
                (:then_1
                  (Game|SpawnActorfromClass "/Game/Blueprints/Resourses/Coal.Coal_C" (Math|Transform|MakeTransform _returnvalue (Math|Rotator|MakeRotator 0.0 0.0 0.0) "1,1,1") "Undefined" 0 0)
                  (Variables|Default|SetDrova3 true)
                  (CallFunction|Ygol)
                  (Variables|/Game/Blueprints/Pechi/Pech.Pech_C|SetYgol _pech true)
                  (Default|DeletePlane _pech))
                (:then_2
                  (Collision|SetCollisionEnabled (Variables|Default|GetCube) "QueryOnly")))))
          (else
            (Rendering|Components|TextRender|SetText _text "No Stone Cast")
            (Default|ActivateAnimation _hand_wid)
            (goto _label Reset)))
        (else
          (Rendering|Components|TextRender|SetText _text "No Tinder-boxes left")
          (Default|ActivateAnimation _hand_wid)
          (goto _label Reset))))))

(fn ConstructionScript)

(fn Ygol
  (return (Variables|Default|GetDrova3)))

(fn ITM
  (return 0 false))